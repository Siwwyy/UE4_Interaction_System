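; Player Blueprint that handles movement, camera look and interaction with objects in the world.
; Axis inputs drive movement along the actor's forward and right vectors and add controller yaw and pitch.
; Interact line-traces from the camera for static and dynamic objects, though its rotated offset is a zero vector, so start equals end.
; A hit box component whose attach parent is an Interactable_Scene_Component calls Trigger on that parent.
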(event Input|ActionEvents|InputActionInteract
  (params (Key :type Key%20Structure :default "None"))
  (bind _camera (Variables|Default|GetCamera))
  (bind _returnvalue (Transformation|GetWorldLocation _camera))
  (:Pressed
    (bind (_outhit _returnvalue_2) (Collision|LineTraceForObjects _returnvalue (+ _returnvalue (Math|Vector|RotateVector (Math|Vector|MakeVector 0.0 0.0 0.0) (Transformation|GetWorldRotation _camera))) (Utilities|Array|MakeArray "ObjectTypeQuery1" "ObjectTypeQuery2") false 0 "None"))
    (if _returnvalue_2
      (bind _asbox_collision (Utilities|Casting|CastToBoxComponent (.HitComponent (Collision|BreakHitResult _outhit))))
      (bind _asinteractable_scene_component (Utilities|Casting|CastToInteractable_Scene_Component (Transformation|GetAttachParent _asbox_collision)))
      (Class|InteractableSceneComponent|Trigger _asinteractable_scene_component))))

(event Input|AxisEvents|InputAxisMoveForward
  (params (AxisValue :type Float%20%28single-precision%29))
  (Pawn|Input|AddMovementInput (Transformation|GetActorForwardVector) AxisValue false))

(event Input|AxisEvents|InputAxisMoveRight
  (params (AxisValue :type Float%20%28single-precision%29))
  (Pawn|Input|AddMovementInput (Transformation|GetActorRightVector) AxisValue false))

(event Input|AxisEvents|InputAxisYaw
  (params (AxisValue :type Float%20%28single-precision%29))
  (Pawn|Input|AddControllerYawInput AxisValue))

(event Input|AxisEvents|InputAxisPitch
  (params (AxisValue :type Float%20%28single-precision%29))
  (Pawn|Input|AddControllerPitchInput AxisValue))

(fn ConstructionScript)